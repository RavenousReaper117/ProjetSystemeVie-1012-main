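; AC_health is a health component that tracks current and max health and a death state for its owner.
; TakeDamage and GainHealth are ignored while dead, whereas ResetHealth clears the dead state and restores max health.
; All three events feed UpdateHealthAndNoticy, which clamps health between zero and max and broadcasts OnHealthChanged.
; When health reaches zero, that function sets IsDead and broadcasts OnDeath.
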(event EventTakeDamage
  (params (DamageAmount :type Float%20%28double-precision%29))
  ;[0.15 0.15 0.15 0.5] Take Damage
  (if (not (Variables|Default|GetIsDead))
    (CallFunction|UpdateHealthandNoticy (- (Variables|Default|GetCurrentHealth) DamageAmount))))

(event EventGainHealth
  (params (HealthAmount :type Float%20%28double-precision%29))
  ;[0.15 0.15 0.15 0.5] Gain health
  (if (not (Variables|Default|GetIsDead))
    (CallFunction|UpdateHealthandNoticy (+ (Variables|Default|GetCurrentHealth) HealthAmount))))

(event EventResetHealth
  ;[0.15 0.15 0.15 0.5] Reset health
  (Variables|Default|SetIsDead false)
  (CallFunction|UpdateHealthandNoticy (Variables|Default|GetMaxHealth)))

(fn UpdateHealthandNoticy
  (params (NewHealthValue :type Float%20%28double-precision%29))
  (bind _maxhealth (Variables|Default|GetMaxHealth))
  (bind _output_get (Variables|Default|SetCurrentHealth (Math|Float|Clamp(Float) NewHealthValue 0.0 _maxhealth)))
  (Default|CallOnHealthChanged _output_get _maxhealth)
  (if (<= (Variables|Default|GetCurrentHealth) 0.0)
    (Variables|Default|SetIsDead true)
    (Default|CallOnDeath)
    (else
      (Variables|Default|SetIsDead false))))