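; Player state that keeps the player's health across levels and triggers respawn on death.
; On begin play it restores health from BP_GameInstance, or resets the health component the first time and flags it as initialized.
; Every health change event from the component writes current and max health back to the game instance.
; On death it asks BP_ThirdPersonGameMode to start respawning player controller 0.
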(event OnHealthChanged(AC_health)
  (params (CurrentHealth :type Float%20%28double-precision%29) (MaxHealth :type Float%20%28double-precision%29))
  ;[0.15 0.15 0.15 0.5] Lors de nimportequel changement de vie, je save dans player state les stats
  (CallFunction|SaveCurrentHealth CurrentHealth)
  (CallFunction|SaveMaxHealth MaxHealth))

(event OnDeath(AC_health)
  ;[0.15 0.15 0.15 0.5] Respawn lors de la mort
  (bind _asbp_third_person_game_mode (Utilities|Casting|CastToBP_ThirdPersonGameMode (Game|GetGameMode)))
  (Default|StartRespawn _asbp_third_person_game_mode (Game|GetPlayerController 0)))

(event EventBeginPlay
  ;[0.15 0.15 0.15 0.5] Référence du game instance qui va servir a stocker les valeurs de la vie
  (bind _asbp_game_instance (Utilities|Casting|CastToBP_GameInstance (Game|GetGameInstance)))
  (bind _output_get (Variables|Default|SetREF%20BPGameInstance _asbp_game_instance))
  (if (Variables|/Game/Game/Blueprints/BP_GameInstance.BP_GameInstance_C|GetHealthInitialized_GI _output_get)
    (CallFunction|LoadHealthfromGameInstance)
    (else
      (Default|ResetHealth (Variables|Default|GetAC_health))
      (Variables|/Game/Game/Blueprints/BP_GameInstance.BP_GameInstance_C|SetHealthInitialized_GI (Variables|Default|GetREF%20BPGameInstance) true))))

(fn ConstructionScript)

(fn SaveCurrentHealth
  (params (NewHealth :type Float%20%28double-precision%29))
  (Variables|/Game/Game/Blueprints/BP_GameInstance.BP_GameInstance_C|SetCurrentHealth_GI (Variables|Default|GetREF%20BPGameInstance) NewHealth))

(fn SaveMaxHealth
  (params (NewMaxHealth :type Float%20%28double-precision%29))
  (Variables|/Game/Game/Blueprints/BP_GameInstance.BP_GameInstance_C|SetMaxHealth_GI (Variables|Default|GetREF%20BPGameInstance) NewMaxHealth))

(fn LoadHealthfromGameInstance
  ;[0.15 0.15 0.15 0.5] Je prends les valeurs du game instance pour mettre à jour la vie du joueur dans un nouveau niveau
  (bind _output_get (Variables|/Game/Game/Blueprints/Components/AC_health.AC_health_C|SetMaxHealth (Variables|Default|GetAC_health) (Variables|/Game/Game/Blueprints/BP_GameInstance.BP_GameInstance_C|GetMaxHealth_GI (Variables|Default|GetREF%20BPGameInstance))))
  (bind _output_get_2 (Variables|/Game/Game/Blueprints/Components/AC_health.AC_health_C|SetCurrentHealth (Variables|Default|GetAC_health) (Variables|/Game/Game/Blueprints/BP_GameInstance.BP_GameInstance_C|GetCurrentHealth_GI (Variables|Default|GetREF%20BPGameInstance))))
  (Default|CallOnHealthChanged (Variables|Default|GetAC_health) _output_get_2 _output_get))